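; Game mode for the tile game that sets up the on-screen UI and provides a map reset.
; On BeginPlay it adds the player HUD widget to the viewport, plus a debug widget layered above it in non-Shipping builds.
; ResetMap restarts the map by reopening the current level by name.
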(event `self.ReceiveBeginPlay`
  (bind _returnvalue (`|CreateWidget` "/Game/UI/Blueprints/PlayerHUDWidget.PlayerHUDWidget_C"))
  (`UserWidget.AddToViewport` _returnvalue 0)
  ;[0 0 0 1 14] If the build is NOT a "Shipping" build, spawn the debug UI
  (if (!= "Shipping" (`KismetSystemLibrary.GetBuildConfiguration`))
    (bind _returnvalue_2 (`|CreateWidget` "/Game/UI/Blueprints/UI_Debug.UI_Debug_C"))
    (`UserWidget.AddToViewport` _returnvalue_2 100)))

(fn `ResetMap`
  (bind _returnvalue (`GameplayStatics.GetCurrentLevelName` true))
  (`GameplayStatics.OpenLevel` (`KismetStringLibrary.Conv_StringToName` _returnvalue)))

(fn `UserConstructionScript`)