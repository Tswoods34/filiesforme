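; Base grid Entity that moves smoothly between tiles through the MovetoTile event.
; A move starts only for a valid, enterable tile while not already moving, then notifies the old tile via OnExit and immediately claims the destination by clearing CanEnter.
; A timeline lerps the actor between tile locations, optionally hidden during travel.
; On finish it restores visibility if it hid the actor, clears IsMoving and fires the new tile's OnEntered.
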(event `Move to Tile`
  (params (`Destination Tile` :type "/Game/Blueprints/Tiles/Tile Object Reference") (`Move Invisibly` :type Boolean))
  ;[0 0 0 1 14] If target tile is valid, and target tile is enterable, and the player is not already moving, set IsMoving to true and begin the moving process
  (`/Engine/EditorBlueprintResources/StandardMacros.IsValid` `Destination Tile`
    (:`Is Valid`
      (if (and (`/Game/Blueprints/Tiles/Tile.CanEnter` `Destination Tile`) (not (`self.IsMoving`)))
        (set `self.IsMoving` true)
        (`self.SetActorHiddenInGame` `Move Invisibly`)
        ;[0 0 0 1 14] Call On Exit event for current tile
        (`/Game/Blueprints/Tiles/Tile.On Exit` (`self.CurrentTile`) `Destination Tile` self)
        ;[0 0 0 1 14] Assign Current Tile as Previous Tile and Target Tile as Current Tile
        (set `self.PreviousTile` (`self.CurrentTile`))
        (bind _output_get (set `self.CurrentTile` `Destination Tile`))
        ;[0 0 0 1 14] "Claim" the tile we are about to enter so nothing attempts to enter it as we animate.
        (set `/Game/Blueprints/Tiles/Tile.CanEnter` false _output_get)
        ;[0 0 0 1 14] Timeline and Lerp for smooth movement instead of visually teleporting
        (bind (_direction _move_progress) (`Timeline|Timeline_0` :!via `PlayFromStart`)
          (:`Update`
            ;[0 0 0 1 14] This actually moves the player pawn
            (`self.K2_SetActorLocation` (`KismetMathLibrary.VLerp` (`self.K2_GetActorLocation` (`self.PreviousTile`)) (`self.K2_GetActorLocation` (`self.CurrentTile`)) _move_progress)))
          (:`Finished`
            ;[0 0 0 1 14] If MoveInvisibly was true, ensure the object is visible again.
            (if `Move Invisibly`
              (`self.SetActorHiddenInGame` false))
            (set `self.IsMoving` false)
            ;[0 0 0 1 14] Call On Entered event for new Current Tile
            (`/Game/Blueprints/Tiles/Tile.On Entered` (`self.CurrentTile`) (`self.PreviousTile`) self)))))))

(fn `UserConstructionScript`)