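; Grid tile actor for a TileMap that tracks its occupying entity and whether it can be entered.
; Enter and exit events maintain occupancy, while neighbor queries add direction deltas to its coordinate, with a guard against a build-only invalid direction.
; UpdateTile, also exposed through an editor wrapper, replaces the tile with a newly spawned type at its map coordinate.
; Both update functions can swap the occupant but never destroy the player.
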(event `On Entered`
  (params (`Previous Tile` :type "/Game/Blueprints/Tiles/Tile Object Reference") (`Entering Entity` :type "/Game/Blueprints/Entities/Entity Object Reference"))
  (if (`KismetSystemLibrary.IsValid` `Entering Entity`)
    (set `self.CanEnter` false)
    (set `self.CurrentEntity` `Entering Entity`)
    (else
      (`KismetSystemLibrary.PrintString` "Tile: An invalid object attempted to enter this tile!" true true (struct :`R` 1.0 :`A` 1.0) 8.0))))

(event `On Exit`
  (params (`Destination Tile` :type "/Game/Blueprints/Tiles/Tile Object Reference") (`Exiting Entity` :type "/Game/Blueprints/Entities/Entity Object Reference"))
  (if (`KismetSystemLibrary.IsValid` `Exiting Entity`)
    (set `self.CanEnter` true)
    (set `self.CurrentEntity` null)
    (else
      (`KismetSystemLibrary.PrintString` "Tile: An invalid object attempted to leave this tile!" true true (struct :`R` 1.0 :`A` 1.0) 8.0))))

(fn `GetAllNeighbors`
  (returns (Neighbors :type "Map of /Game/Blueprints/Directions/Direction Object Reference to /Game/Blueprints/Tiles/Tile Object Reference"))
  (return (`|MakeMap` "/Game/Blueprints/Directions/Up.Up" (`self.GetNeighbor` "/Game/Blueprints/Directions/Up.Up") "/Game/Blueprints/Directions/Right.Right" (`self.GetNeighbor` "/Game/Blueprints/Directions/Right.Right") "/Game/Blueprints/Directions/Down.Down" (`self.GetNeighbor` "/Game/Blueprints/Directions/Down.Down") "/Game/Blueprints/Directions/Left.Left" (`self.GetNeighbor` "/Game/Blueprints/Directions/Left.Left") :!type "/Game/Blueprints/Directions/Direction Object Reference")))

(fn `GetNeighbor`
  (params (Direction :type "/Game/Blueprints/Directions/Direction Object Reference"))
  (returns (Neighbor :type "/Game/Blueprints/Tiles/Tile Object Reference") (FoundNeighbor :type Boolean))
  (bind (_x _y) (break `/Game/Blueprints/Coord` (`self.Coord`)))
  (bind (_x_2 _y_2) (break `/Game/Blueprints/Coord` (`/Game/Blueprints/Directions/Direction.Delta` Direction)))
  (bind _tile (`/Game/Blueprints/TileMap.GetTileAtCoord` (`self.TileMap`) (make `/Game/Blueprints/Coord` (+ _x_2 _x) (+ _y_2 _y))))
  (return _tile (`KismetSystemLibrary.IsValid` _tile)))

(fn `IsTileNeighbor?`
  (params (Tile :type "/Game/Blueprints/Tiles/Tile Object Reference"))
  (returns (TileIsNeighbor :type Boolean) (NeighborDirection :type "/Game/Blueprints/Directions/Direction Object Reference"))
  (locals (TileToCheck :type "/Game/Blueprints/Tiles/Tile Object Reference"))
  ;[0 0 0 1 14] Assign Tile being checked as local variable
  (set `local.TileToCheck` Tile)
  ;[0 0 0 1 14] Step through each Neighboring tile
  (bind _values (`BlueprintMapLibrary.Map_Values` (`self.GetAllNeighbors`)))
  (for _array_element _values
    ;[0 0 0 1 14] Is current neighbor equal to tile being checked?
    (if (== (`local.TileToCheck`) _array_element)
      ;[0 0 0 1 14] Step through each direction of neighbors
      (bind _keys (`BlueprintMapLibrary.Map_Keys` (`self.GetAllNeighbors`)))
      (for _array_element_2 _keys
        ;[0 0 0 1 14] If the current direction's tile matches the tile being checked, the tile is a neighbor in that direction, return that direction information
        (if (and (!= _array_element_2 null) (== (`local.TileToCheck`) (`self.GetNeighbor` _array_element_2)))
          (return true _array_element_2)))))
  (return false null) ; If tile is NOT a neighbor
)

(fn `SetAsSpawnTile`
  (`/Game/Blueprints/TileMap.SetSpawnTile` (`self.TileMap`) self))

(fn `Update Entity`
  (returns (NewEntity :type "/Game/Blueprints/Entities/Entity Object Reference"))
  (bind _currententity (`self.CurrentEntity`))
  (`/Engine/EditorBlueprintResources/StandardMacros.IsValid` _currententity
    (:`Is Valid`
      ;[0 0 0 1 14] If CurrentEntity is the player, send warning and exit function
      (bind _asentity_player (cast `/Game/Blueprints/Entities/Player/Entity_Player` _currententity)
        (:`then`
          (if (== _asentity_player (`GameplayStatics.GetPlayerPawn` 0))
            (`KismetSystemLibrary.PrintString` "Tile - UpdateTileType: The player is on the tile you are updating, so we cannot spawn the desired Entity!" true true (struct :`R` 1.0 :`A` 1.0) 16.0)
            (return null)
            (else
              _)))
        (:`CastFailed`
          _))
      ;[0 0 0 1 14] If CurrentEntity is not the player then destroy it.
      (`self.K2_DestroyActor` (`self.CurrentEntity`)))
    (:`Is Not Valid`
      _))
  ;[0 0 0 1 14] If NewEntityType is not null, then we should be generating a new Entity!
  (if (== (`self.NewEntityType`) null)
    (set `self.CanEnter` true)
    (set `self.CurrentEntity` null)
    (return null)
    (else
      ;[0 0 0 1 14] Spawn new Entity, Set its current tile this tile, set this tile's variables to appropriate values
      (bind _returnvalue (`|SpawnActorFromClass` (`self.NewEntityType`) (`self.GetTransform`) "Undefined" "SelectDefaultAtRuntime" null self null))
      (if (`KismetSystemLibrary.IsValid` _returnvalue)
        (set `self.CurrentEntity` _returnvalue)
        (set `self.CanEnter` false)
        (return _returnvalue)
        (else
          (`KismetSystemLibrary.PrintString` "Tile - UpdateTileType: The spawned actor is not valid! How is this possible?" true true (struct :`R` 1.0 :`A` 1.0) 8.0))))))

(fn `Update Tile`
  (returns (NewTile :type "/Game/Blueprints/Tiles/Tile Object Reference"))
  (locals (TempNewTile :type "/Game/Blueprints/Tiles/Tile Object Reference") (PlayerIsPresent :type Boolean))
  (bind _currententity (`self.CurrentEntity`))
  (bind _tempnewtile (`local.TempNewTile`))
  (bind _tempnewtile_2 (`local.TempNewTile`))
  (bind _tilemap (`self.TileMap`))
  (if (== (`self.NewTileType`) null)
    ;[0 0 0 1 15] If we're trying to add an Entity while New Tile Type is empty, set it to our current Tile Type.
    (set `self.NewTileType` (`GameplayStatics.GetObjectClass` self)))
  ;[0 0 0 1 24] Deal with Tile
  ;;[0.2 0.2 0.2] Spawn new tile from type
  (bind _returnvalue (`|SpawnActorFromClass` (`self.NewTileType`) (`self.GetTransform`) "Undefined" "SelectDefaultAtRuntime" null (`self.TileMap`) (`/Game/Blueprints/TileMap.IndexToCoord` _tilemap (`KismetArrayLibrary.Array_Find` (`/Game/Blueprints/TileMap.Tiles` _tilemap) self)) null))
  (set `local.TempNewTile` _returnvalue)
  ;;[0.2 0.2 0.2] Replace the tile in the tile map
  (`/Game/Blueprints/TileMap.Replace Tile` (`self.TileMap`) (`local.TempNewTile`))
  (`self.K2_AttachToActor` (`local.TempNewTile`) (`self.TileMap`) "None" "KeepWorld" "KeepWorld" "KeepWorld" true)
  ;[0 0 0 1 24] Deal with Entity & Player
  (`/Engine/EditorBlueprintResources/StandardMacros.IsValid` _currententity
    (:`Is Valid`
      ;;[0.2 0.2 0.2] If CurrentEntity is the player, move player safely onto new tile if it is enterable.
      (bind _asentity_player (cast `/Game/Blueprints/Entities/Player/Entity_Player` _currententity)
        (:`then`
          (if (== _asentity_player (`GameplayStatics.GetPlayerPawn` 0))
            (set `local.PlayerIsPresent` true)
            (if (`/Game/Blueprints/Tiles/Tile.CanEnter` (`local.TempNewTile`))
              (set `/Game/Blueprints/Entities/Entity.CurrentTile` _tempnewtile_2 _asentity_player)
              (`self.On Entered` _tempnewtile_2 null _asentity_player)
              ;;[0.2 0.2 0.2] If NewEntityType is not null, then we should be generating a new Entity!
              (if (== (`self.NewEntityType`) null) :!label _label
                (`self.K2_DestroyActor` :!label _label_2)
                (return (`local.TempNewTile`))
                (elif (`local.PlayerIsPresent`)
                  (`KismetSystemLibrary.PrintString` "Tile - UpdateTileType: The player is on the tile you are updating, so we cannot spawn the desired Entity!" true true (struct :`R` 1.0 :`A` 1.0) 16.0)
                  (goto _label_2)
                  (else
                    ;;[0.2 0.2 0.2] Spawn new Entity, Set its current tile to the new tile, set new tile's variables to appropriate values
                    (bind _returnvalue_2 (`|SpawnActorFromClass` (`self.NewEntityType`) (`self.GetTransform`) "Undefined" "SelectDefaultAtRuntime" null (`local.TempNewTile`) null))
                    (if (`KismetSystemLibrary.IsValid` _returnvalue_2)
                      (set `/Game/Blueprints/Tiles/Tile.CurrentEntity` _returnvalue_2 _tempnewtile)
                      (set `/Game/Blueprints/Tiles/Tile.CanEnter` false _tempnewtile)
                      (goto _label_2)
                      (else
                        (`KismetSystemLibrary.PrintString` "Tile - UpdateTileType: The spawned actor is not valid! How is this possible?" true true (struct :`R` 1.0 :`A` 1.0) 8.0))))))
              (else
                (`KismetSystemLibrary.PrintString` "Tile - UpdateTileType: The player is on the tile you are updating, but cannot be put onto the new tile!" true true (struct :`R` 1.0 :`A` 1.0) 16.0)))
            (else
              ;;[0.2 0.2 0.2] If CurrentEntity is not the player, destroy whatever it is.
              (`self.K2_DestroyActor` (`self.CurrentEntity`) :!label _label_3)
              (goto _label))))
        (:`CastFailed`
          (goto _label_3))))
    (:`Is Not Valid`
      (goto _label))))

(fn `Update Tile (in Editor)`
  (`self.Update Tile`))

(fn `UserConstructionScript`)