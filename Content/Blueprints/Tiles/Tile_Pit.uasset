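; Pit tile that swallows any entity entering it, killing the player or removing any other entity.
; On entry it disables the entity's input and lowers it by FallDistance with a timeline before resolving its fate, clearing non-players through UpdateEntity.
; At BeginPlay it checks its four neighbours and shows a wall only beside existing non-pit tiles, so adjacent pits read as one hole.
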(event `self.ReceiveBeginPlay`
  (`parent.ReceiveBeginPlay`)
  (`self.AdjustWallVisibility`))

(event `self.On Entered`
  (params (`Previous Tile` :type "/Game/Blueprints/Tiles/Tile Object Reference") (`Entering Entity` :type "/Game/Blueprints/Entities/Entity Object Reference"))
  (bind _currententity (`self.CurrentEntity`))
  (`parent.On Entered` `Previous Tile` `Entering Entity`)
  (`self.DisableInput` _currententity null)
  (bind _output_get (set `self.StartPos` (`self.K2_GetActorLocation` _currententity)))
  (set `self.EndPos` (- _output_get (`KismetMathLibrary.MakeVector` 0.0 0.0 (`self.Fall Distance`))))
  (bind (_direction _alpha) (`Timeline|Falling Animation` :!via `PlayFromStart`)
    (:`Update`
      (`self.K2_SetActorLocation` (`self.CurrentEntity`) (`KismetMathLibrary.VLerp` (`self.StartPos`) (`self.EndPos`) _alpha) false false))
    (:`Finished`
      ;[0 0 0 1 14] If the entity is the player, reset the level.
      (bind _asentity_player (cast `/Game/Blueprints/Entities/Player/Entity_Player` (`self.CurrentEntity`))
        (:`then`
          (`/Game/Blueprints/Entities/Player/Entity_Player.KillPlayer` _asentity_player))
        (:`CastFailed`
          ;[0 0 0 1 14] If entity is not the players, simply destroy the entity.
          (set `self.NewEntityType` null)
          (`self.Update Entity`))))))

(fn `AdjustWallVisibility`
  (`self.NewMacro_0` (`self.WallUp`) "/Game/Blueprints/Directions/Up.Up")
  (`self.NewMacro_0` (`self.WallRight`) "/Game/Blueprints/Directions/Right.Right")
  (`self.NewMacro_0` (`self.WallDown`) "/Game/Blueprints/Directions/Down.Down")
  (`self.NewMacro_0` (`self.WallLeft`) "/Game/Blueprints/Directions/Left.Left"))

(fn `UserConstructionScript`
  (`parent.UserConstructionScript`))