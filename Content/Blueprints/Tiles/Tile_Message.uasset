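; Message tile that shows world-space text when a player or interactable entity enters it, with separate messages for each.
; On BeginPlay it colors the text widget orange, disables its shadow and rotates it toward the tile map's camera.
; The text hides on exit, or optionally after a retriggerable delay.
; Its CanPlayerEnter check always returns false, despite OnEntered handling players.
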(event `self.ReceiveBeginPlay`
  (`parent.ReceiveBeginPlay`)
  ;[0 0 0 1 14] Set Text Color to match material
  (bind _asworld_text_widget (cast `/Game/UI/Blueprints/WorldTextWidget` (`WidgetComponent.GetWidget` (`self.TextWidget`))))
  (`/Game/UI/Blueprints/WorldTextWidget.SetTextColor` _asworld_text_widget (struct :`R` 1.0 :`G` 0.4 :`A` 1.0))
  (`PrimitiveComponent.SetCastShadow` (`self.TextWidget`) false) ; Normally this would be set in the details panel\nof the component, but for some reason widget\ncomponents do not have the value propery exposed.
  ;[0 0 0 1 14] Rotate the TextWidget so it is facing the camera.
  (`SceneComponent.K2_SetWorldRotation` (`self.TextWidget`) (`KismetMathLibrary.Conv_VectorToRotator` (`KismetMathLibrary.Normal` (- (`self.K2_GetActorLocation` (`/Game/Blueprints/TileMap.CameraActor` (`self.TileMap`))) (`SceneComponent.K2_GetComponentLocation` (`self.TextWidget`))))) false false))

(event `self.On Entered`
  (params (`Previous Tile` :type "/Game/Blueprints/Tiles/Tile Object Reference") (`Entering Entity` :type "/Game/Blueprints/Entities/Entity Object Reference"))
  (`parent.On Entered` `Previous Tile` `Entering Entity`)
  ;[0 0 0 1 14] Run code conditionally, depending on what type of object just entered!
  (cast `/Game/Blueprints/Entities/Player/Entity_Player` `Entering Entity`
    (:`then`
      (bind _asworld_text_widget (cast `/Game/UI/Blueprints/WorldTextWidget` (`WidgetComponent.GetWidget` (`self.TextWidget`))))
      (`/Game/UI/Blueprints/WorldTextWidget.SetText` _asworld_text_widget (`self.PlayerMessage`)))
    (:`CastFailed`
      (cast `/Game/Blueprints/Entities/Interactables/Entity_Interactable` `Entering Entity`)
      (bind _asworld_text_widget_2 (cast `/Game/UI/Blueprints/WorldTextWidget` (`WidgetComponent.GetWidget` (`self.TextWidget`))))
      (`/Game/UI/Blueprints/WorldTextWidget.SetText` _asworld_text_widget_2 (`self.InteractableMessage`))))
  (`SceneComponent.SetHiddenInGame` (`self.TextWidget`) false true)
  (if (`self.DoesMessageDisappear`)
    (`KismetSystemLibrary.RetriggerableDelay` (`self.DelayBeforeDisappear`))
    (`SceneComponent.SetHiddenInGame` (`self.TextWidget`) true true)))

(event `self.On Exit`
  (params (`Destination Tile` :type "/Game/Blueprints/Tiles/Tile Object Reference") (`Exiting Entity` :type "/Game/Blueprints/Entities/Entity Object Reference"))
  (`parent.On Exit` `Destination Tile` `Exiting Entity`)
  (`SceneComponent.SetHiddenInGame` (`self.TextWidget`) true true))

(fn `CanPlayerEnter?`
  (params (Player :type "/Game/Blueprints/Entities/Player/Entity_Player Object Reference") (From :type "/Game/Blueprints/Tiles/Tile Object Reference"))
  (returns (`Can Enter` :type Boolean))
  (return false))

(fn `UserConstructionScript`
  (`parent.UserConstructionScript`))