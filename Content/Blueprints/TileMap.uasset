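; TileMap is a grid map actor that owns the level's tiles and places the player on it.
; GenerateMap destroys old tiles and their entities, then spawns attached border and fill tiles into a flat, row-major array.
; Coordinate helpers handle index conversion, bounds checks, lookup and replacement in that array.
; On BeginPlay it sets the camera, moves the player to the spawn tile, sets facing and marks that tile occupied and not enterable.
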(event `self.ReceiveBeginPlay`
  (bind _returnvalue (`GameplayStatics.GetPlayerPawn` 0))
  (bind _playerspawntile (`self.PlayerSpawnTile`))
  (bind _playerspawntile_2 (`self.PlayerSpawnTile`))
  ;[0 0 0 1 14] Set Main Camera
  (`PlayerController.SetViewTargetWithBlend` (`GameplayStatics.GetPlayerController` 0) (`self.CameraActor`) 0.0 "VTBlend_Linear" 0.0 false)
  ;[0 0 0 1 14] Spawn Player
  (`/Engine/EditorBlueprintResources/StandardMacros.IsValid` _playerspawntile
    (:`Is Valid`
      (`self.K2_SetActorLocation` _returnvalue (`self.K2_GetActorLocation` _playerspawntile) false false)
      ;[0 0 0 1 14] Initialize Variables on Player, Make Player Spawn Tile Not Enterable
      (bind _asentity_player (cast `/Game/Blueprints/Entities/Player/Entity_Player` _returnvalue))
      (set `/Game/Blueprints/Entities/Entity.CurrentTile` _playerspawntile_2 _asentity_player)
      (set `/Game/Blueprints/Tiles/Tile.CanEnter` false _playerspawntile_2)
      (set `/Game/Blueprints/Tiles/Tile.CurrentEntity` _asentity_player _playerspawntile_2)
      (`/Game/Blueprints/Entities/Player/Entity_Player.Face Direction` _asentity_player (`self.PlayerSpawnDirection`)))
    (:`Is Not Valid`
      (`KismetSystemLibrary.PrintString` "TileMap: No Player Spawn Tile is set!" true true (struct :`R` 1.0 :`A` 1.0) 16.0))))

(fn `CoordToIndex`
  (params (Coord :type "/Game/Blueprints/Coord Structure"))
  (returns (Index :type Integer))
  (return (+ Coord_X_5_6F435FC24D9202AE27D58A9D538EE86B (* Coord_Y_7_1CB6DBA146075157CAA02385B7A6DC31 (`self.Width`)))))

(fn `GenerateMap`
  (for _array_element (`self.Tiles`)
    ;[0 0 0] Loop Body
    (`/Engine/EditorBlueprintResources/StandardMacros.IsValid` _array_element
      (:`Is Valid`
        (bind _currententity (`/Game/Blueprints/Tiles/Tile.CurrentEntity` _array_element))
        ;;[0.2 0.2 0.2 1 14] If current Entity is NOT null, destroy it
        (if (!= _currententity null)
          (`self.K2_DestroyActor` _currententity))
        (`self.K2_DestroyActor` _array_element) ; Destroy Tile
      )))
  (`KismetArrayLibrary.Array_Clear` (`self.Tiles`))
  (for _index (range (`self.Height`))
    (for _index_2 (range (`self.Width`))
      (bind _returnvalue (`|SpawnActorFromClass` (select `bool` (`self.IsCoordOnBorder` (make `/Game/Blueprints/Coord` _index_2 _index)) :`false` (`self.FillTileType`) :`true` (`self.BorderTileType`)) (`KismetMathLibrary.MakeTransform` (`KismetMathLibrary.MakeVector` (* _index 100.0) (* _index_2 100.0))) "Undefined" "SelectDefaultAtRuntime" null self (make `/Game/Blueprints/Coord` _index_2 _index) null))
      (`KismetArrayLibrary.Array_Add` (`self.Tiles`) _returnvalue)
      (`self.K2_AttachToActor` _returnvalue self "None" "KeepWorld" "KeepWorld" "KeepWorld" true))))

(fn `GetTileAtCoord`
  (params (Coord :type "/Game/Blueprints/Coord Structure"))
  (returns (Tile :type "/Game/Blueprints/Tiles/Tile Object Reference"))
  (return (`|GetArrayItem` (`self.Tiles`) (`self.CoordToIndex` Coord))))

(fn `IndexToCoord`
  (params (Index :type Integer))
  (returns (Coord :type "/Game/Blueprints/Coord Structure"))
  (bind _width (`self.Width`))
  (return (make `/Game/Blueprints/Coord` (mod Index _width) (/ Index _width))))

(fn `IsCoordInRange`
  (params (Coord :type "/Game/Blueprints/Coord Structure"))
  (returns (`Is In Range?` :type Boolean))
  (return (not (or (< Coord_X_5_6F435FC24D9202AE27D58A9D538EE86B 0) (< Coord_Y_7_1CB6DBA146075157CAA02385B7A6DC31 0) (>= Coord_X_5_6F435FC24D9202AE27D58A9D538EE86B (`self.Width`)) (>= Coord_Y_7_1CB6DBA146075157CAA02385B7A6DC31 (`self.Height`))))))

(fn `IsCoordOnBorder`
  (params (Coord :type "/Game/Blueprints/Coord Structure"))
  (returns (IsOnBorder :type Boolean))
  (return (or (== Coord_X_5_6F435FC24D9202AE27D58A9D538EE86B 0) (== Coord_X_5_6F435FC24D9202AE27D58A9D538EE86B (- (`self.Width`) 1)) (== Coord_Y_7_1CB6DBA146075157CAA02385B7A6DC31 0) (== Coord_Y_7_1CB6DBA146075157CAA02385B7A6DC31 (- (`self.Height`) 1)))))

(fn `Replace Tile`
  (params (`New Tile` :type "/Game/Blueprints/Tiles/Tile Object Reference"))
  (`KismetArrayLibrary.Array_Set` (`self.Tiles`) (`self.CoordToIndex` (`/Game/Blueprints/Tiles/Tile.Coord` `New Tile`)) `New Tile`))

(fn `SetSpawnTile`
  (params (`Tile To Set` :type "/Game/Blueprints/Tiles/Tile Object Reference"))
  (set `self.PlayerSpawnTile` `Tile To Set`))

(fn `UserConstructionScript`)